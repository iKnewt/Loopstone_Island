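; Frog disco Blueprint for the Tavern building that flashes its point lights between blue and pink.
; On BeginPlay it colors two groups of point lights with opposite colors, then swaps the colors after each short delay.
; The loop body wires back into the loop's start, so the alternation repeats indefinitely without using Tick, regardless of the loop's count.
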(event `self.ReceiveBeginPlay`
  (set `self.Color1` (struct :`R` 0.037358 :`B` 1.0 :`A` 1.0))
  (set `self.Color2` (struct :`R` 1.0 :`B` 0.66237 :`A` 1.0))
  (for _ (range 101) :!label _label
    (`KismetSystemLibrary.Delay` 0.4)
    (`LightComponent.SetLightColor` (`self.PointLight`) (`self.Color1`) true)
    (`LightComponent.SetLightColor` (`self.PointLight11`) (`self.Color1`) true)
    (`LightComponent.SetLightColor` (`self.PointLight9`) (`self.Color1`) true)
    (`LightComponent.SetLightColor` (`self.PointLight7`) (`self.Color1`) true)
    (`LightComponent.SetLightColor` (`self.PointLight2`) (`self.Color1`) true)
    (`LightComponent.SetLightColor` (`self.PointLight6`) (`self.Color2`) true)
    (`LightComponent.SetLightColor` (`self.PointLight8`) (`self.Color2`) true)
    (`LightComponent.SetLightColor` (`self.PointLight10`) (`self.Color2`) true)
    (`LightComponent.SetLightColor` (`self.PointLight1`) (`self.Color2`) true)
    (bind _output_get (set `self.ColorTemp` (`self.Color1`)))
    (set `self.Color1` (`self.Color2`))
    (set `self.Color2` _output_get)
    (goto _label)))

(fn `UserConstructionScript`)