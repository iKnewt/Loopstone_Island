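; BP_Cloud is a sky cloud actor that orbits on a spring arm and changes size as it travels.
; BeginPlay gives the mesh a random rotation for variety.
; Each tick pitches the arm at a set speed and applies the opposite pitch to the mesh to offset the orbital spin.
; A float curve sampled with the arm's world pitch sets the mesh's uniform world scale.
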(event `self.ReceiveBeginPlay`
  (`SceneComponent.K2_SetRelativeRotation` (`self.StaticMesh`) (`KismetMathLibrary.RandomRotator` false) false false))

(event `self.ReceiveTick`
  (params (DeltaSeconds :type "Float (single-precision)"))
  (bind (_returnvalue_roll _returnvalue_pitch) (`KismetMathLibrary.BreakRotator` (`SceneComponent.K2_GetComponentRotation` (`self.SpringArm`))))
  (bind _returnvalue (* DeltaSeconds (`self.NewVar_0`)))
  (bind _returnvalue_2 (`CurveFloat.GetFloatValue` (`self.NewVar_1`) _returnvalue_pitch))
  (`SceneComponent.K2_AddWorldRotation` (`self.SpringArm`) (`KismetMathLibrary.MakeRotator` 0.0 _returnvalue) false false)
  (`SceneComponent.K2_AddWorldRotation` (`self.StaticMesh`) (`KismetMathLibrary.MakeRotator` 0.0 (* _returnvalue -1.0)) false false)
  (`SceneComponent.SetWorldScale3D` (`self.StaticMesh`) (`KismetMathLibrary.MakeVector` _returnvalue_2 _returnvalue_2 _returnvalue_2)))

(fn `UserConstructionScript`)