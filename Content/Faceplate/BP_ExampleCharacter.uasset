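; Example character Blueprint that tests changing facial expressions on its CharacterFace component.
; On BeginPlay it creates a dynamic material instance from the face's first material, stores it as MouthMaterial and applies it back to that slot.
; After a short delay it prints a debug message, increments a counter and calls ChangeFace with that material and a fixed expression.
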(event `self.ReceiveBeginPlay`
  (bind _returnvalue (`KismetMaterialLibrary.CreateDynamicMaterialInstance` (`PrimitiveComponent.GetMaterial` (`self.CharacterFace`) 0)))
  (bind _output_get (set `self.MouthMaterial` _returnvalue))
  (`PrimitiveComponent.SetMaterial` (`self.CharacterFace`) 0 _output_get)
  (`KismetSystemLibrary.Delay` 5.0)
  (`KismetSystemLibrary.PrintString` "IT HAPPENED")
  (`/Engine/EditorBlueprintResources/StandardMacros.IncrementInt` (`self.NewVar_0`)
    (:`  `
      (`/Game/Faceplate/BPFL_FaceAndMouthTemplates.ChangeFace` (`self.MouthMaterial`) "NewEnumerator18"))))

(fn `UserConstructionScript`)