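; BP_LoopstoneMachine is an environment object that displays loopstones on a spinning base and plays their sound.
; DisplayLoopstone takes a story and a hide flag, toggling all three stones for Detective or one each for Party Planner, Assistant Chef and None.
; PlayLoopstoneSound starts the audio if needed and runs a timeline driving its volume, which replays after a delay.
; Tick continuously rotates the base around its roll axis.
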(event `self.DisplayLoopstone`
  (params (story :type "EStory Enum" :default "Detective") (HideStone :type Boolean))
  (switch `EStory` story
    (:`Detective`
      (`SceneComponent.SetHiddenInGame` (`self.Loopstone`) HideStone false)
      (`SceneComponent.SetHiddenInGame` (`self.Loopstone1`) HideStone false)
      (`SceneComponent.SetHiddenInGame` (`self.Loopstone2`) HideStone false))
    (:`PartyPlanner`
      (`SceneComponent.SetHiddenInGame` (`self.Loopstone`) HideStone false))
    (:`AssistantChef`
      (`SceneComponent.SetHiddenInGame` (`self.Loopstone1`) HideStone false))
    (:`None`
      (`SceneComponent.SetHiddenInGame` (`self.Loopstone2`) HideStone false))))

(event `self.PlayLoopstoneSound`
  (bind _sound (`self.Sound`))
  (if (`AudioComponent.IsPlaying` _sound)
    (bind (_direction _newtrack_0) (`Timeline|Timeline_0` :!via `PlayFromStart` :!label _label)
      (:`Update`
        (`AudioComponent.SetVolumeMultiplier` (`self.Sound`) _newtrack_0))
      (:`Finished`
        (`KismetSystemLibrary.Delay` 5.0)
        (goto _label :!via `PlayFromStart`)))
    (else
      (`AudioComponent.Play` _sound 0.0)
      (goto _label :!via `PlayFromStart`))))

(event `self.ReceiveTick`
  (params (DeltaSeconds :type "Float (single-precision)"))
  (`SceneComponent.K2_AddRelativeRotation` (`self.LoopstoneBase`) (`KismetMathLibrary.MakeRotator` (* DeltaSeconds -20.0)) false false))

(fn `UserConstructionScript`)