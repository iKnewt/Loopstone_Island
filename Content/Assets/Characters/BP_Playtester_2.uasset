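; BP_Playtester_2 is a playtester actor that is visible and collidable only when the player's developer mode is on.
; On BeginPlay, after calling the parent, it casts player 0's character to BP_PlayerCharacter and uses DevMode to set visibility and collision.
; If the cast fails, it stays hidden with collision disabled.
; DevMode is read only once, so later changes to it are not reflected.
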(event `self.ReceiveBeginPlay`
  (`parent.ReceiveBeginPlay`)
  (bind _asbp_player_character (cast `/Game/Assets/Characters/Player/BP_PlayerCharacter` (`GameplayStatics.GetPlayerCharacter` 0))
    (:`then`
      (bind _devmode (`/Game/Assets/Characters/Player/BP_PlayerCharacter.DevMode` _asbp_player_character))
      (`self.SetActorHiddenInGame` (not _devmode))
      (`self.SetActorEnableCollision` _devmode))
    (:`CastFailed`
      (`self.SetActorHiddenInGame` true)
      (`self.SetActorEnableCollision` false))))

(fn `UserConstructionScript`
  (`parent.UserConstructionScript`))