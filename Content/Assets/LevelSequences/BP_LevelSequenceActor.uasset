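; Helper actor exposing gameplay events for level sequences around loopstone collection and the day loop.
; GoToBed shows the credits widget once the game state reports all loopstones collected, otherwise it opens the Fullday level.
; ShowLoopstone spawns and sets up a loopstone room below the origin.
; CheckIfLastLoopstone returns the view to the player, collects the current story's loopstone and restores walking; StopAllMusic forwards to the game state.
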(event `GoToBed`
  (bind _asloopstone_island_game_state (cast `Loopstone_IslandGameState` (`GameplayStatics.GetGameState`)))
  (bind _returnvalue (`Loopstone_IslandGameState.HasCollectedAllLoopstones` _asloopstone_island_game_state))
  (if _returnvalue
    (bind _returnvalue_2 (`|CreateWidget` "/Game/Assets/UI/WBP_Credits.WBP_Credits_C"))
    (`UserWidget.AddToViewport` _returnvalue_2 0)
    (else
      (`GameplayStatics.OpenLevel` "Fullday"))))

(event `ShowLoopstone`
  (bind _returnvalue (`|SpawnActorFromClass` "/Game/Assets/Environment/Objects/Loopstone/BP_LoopstoneRoom.BP_LoopstoneRoom_C" (`KismetMathLibrary.MakeTransform` (0.0 0.0 -700.0)) "Undefined" "OverrideRootScale" null null))
  (`/Game/Assets/Environment/Objects/Loopstone/BP_LoopstoneRoom.Setup` _returnvalue))

(event `CheckIfLastLoopstone`
  (`PlayerController.SetViewTargetWithBlend` (`GameplayStatics.GetPlayerController` 0) (`GameplayStatics.GetPlayerCharacter` 0) 0.0 "VTBlend_Linear" 0.0 false)
  (bind _asloopstone_island_game_state (cast `Loopstone_IslandGameState` (`GameplayStatics.GetGameState`)))
  (`Loopstone_IslandGameState.CollectLoopstone` _asloopstone_island_game_state (`Loopstone_IslandGameState.CurrentStory` _asloopstone_island_game_state))
  (`CharacterMovementComponent.SetMovementMode` (`Character.CharacterMovement` (`GameplayStatics.GetPlayerCharacter` 0)) "MOVE_Walking" 0))

(event `StopAllMusic`
  (bind _asbp_loopstone_game_state (cast `/Game/Assets/Core/BP_LoopstoneGameState` (`GameplayStatics.GetGameState`)))
  (`Loopstone_IslandGameState.StopAllMusic` _asbp_loopstone_game_state))

(fn `UserConstructionScript`)