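; Player character Blueprint for Loopstone Island that handles debug-style keys, pausing and an optional wake-up intro.
; BeginPlay, when WakeUp is set, plays the wake-up cutscene sequence with movement and look input disabled.
; Number keys 1–4 switch time of day through the game state, O teleports to a fixed spot, and M opens a settings example widget.
; The Pause input action adds the pause screen widget to the viewport.
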(event `Key|One`
  (params (Key :type "Key Structure"))
  (:`Pressed`
    (set `self.NewTime` "Morning")
    (bind _asloopstone_island_game_state (cast `Loopstone_IslandGameState` (`GameplayStatics.GetGameState`) :!label _label))
    (`Loopstone_IslandGameState.ChangeTimeOfDay` _asloopstone_island_game_state (`self.NewTime`))))

(event `Key|Two`
  (params (Key :type "Key Structure"))
  (:`Pressed`
    (set `self.NewTime` "Afternoon")
    (goto _label)))

(event `Key|Three`
  (params (Key :type "Key Structure"))
  (:`Pressed`
    (set `self.NewTime` "Evening")
    (goto _label)))

(event `Key|Four`
  (params (Key :type "Key Structure"))
  (:`Pressed`
    (set `self.NewTime` "Night")
    (goto _label)))

(event `Key|M`
  (params (Key :type "Key Structure"))
  (:`Pressed`
    (bind _returnvalue (`|CreateWidget` "/Game/Assets/UI/WTF-Settings-CompleteExample.WTF-Settings-CompleteExample_C"))
    (`UserWidget.AddToViewport` _returnvalue 0)))

(event `Key|O`
  (params (Key :type "Key Structure"))
  (:`Pressed`
    (`self.K2_SetActorLocation` (-2310.0 -2120.0 450.0))))

(event `InputAction|Pause`
  (params (Key :type "Key Structure"))
  (:`Pressed`
    (bind _returnvalue (`|CreateWidget` "/Game/Assets/UI/WBP_PauseScreen.WBP_PauseScreen_C"))
    (`UserWidget.AddToViewport` _returnvalue 0)))

(event `self.ReceiveBeginPlay`
  (if (`self.WakeUp`)
    (bind (_outactor _returnvalue) (`LevelSequencePlayer.CreateLevelSequencePlayer` "/Game/Assets/LS_WakeupCutscene.LS_WakeupCutscene" (make `MovieSceneSequencePlaybackSettings` false (struct) 1.0 0.0 false false true true)))
    (set `self.NewVar_0` _outactor)
    (bind _output_get (set `self.WakeupCutscene` _returnvalue))
    (`MovieSceneSequencePlayer.Play` _output_get)))

(event `self.WakeupCutscene.OnFinished`)

(fn `UserConstructionScript`)