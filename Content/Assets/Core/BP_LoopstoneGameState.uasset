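; Loopstone's game state, hosting two scripted story events: going to bed and teleporting the doctor.
; GotoBed plays the LS_GoToBed level sequence with movement and look input disabled, then stops all music.
; TeleportDoctor waits, shows a fade-to-black widget, moves the passed Doc to a hardcoded location and calls HideSebastian on SebsHouse, printing a bug message if either reference is invalid.
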(event `self.GoToBed`
  (bind (_outactor _returnvalue) (`LevelSequencePlayer.CreateLevelSequencePlayer` "/Game/Assets/LS_GoToBed.LS_GoToBed" (make `MovieSceneSequencePlaybackSettings` false (struct) 1.0 0.0 false false true true)))
  (`MovieSceneSequencePlayer.Play` _returnvalue)
  (`self.StopAllMusic`))

(event `self.TeleportDoctor`
  (params (Doc :type "BaseIslanderCharacter Object Reference"))
  (bind _sebs_house (`self.Sebs House`))
  (`KismetSystemLibrary.Delay` 1.5)
  (bind _returnvalue (`|CreateWidget` "/Game/Assets/UI/WBP_FadeBlack.WBP_FadeBlack_C"))
  (`UserWidget.AddToViewport` _returnvalue 0)
  (`KismetSystemLibrary.Delay` 0.3)
  (`/Engine/EditorBlueprintResources/StandardMacros.IsValid` Doc
    (:`Is Valid`
      (`self.K2_SetActorLocation` Doc (-3551.311279 -3169.0 635.390442) false false)
      (`/Engine/EditorBlueprintResources/StandardMacros.IsValid` _sebs_house
        (:`Is Valid`
          (`/Game/Assets/Environment/Buildings/BP_Building_04_Sebastian.HideSebastian` _sebs_house))
        (:`Is Not Valid`
          (`KismetSystemLibrary.PrintString` "A BUG HAS HAPPENED OH NOO" :!label _label))))
    (:`Is Not Valid`
      (goto _label))))

(fn `UserConstructionScript`)